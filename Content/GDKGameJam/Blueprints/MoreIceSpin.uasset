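; MoreIceSpin is a health pickup that bobs in place until the third-person character collides with it.
; Two timelines, one played forward and the other in reverse, alternate endlessly to drive the relative location of component E for the floating motion.
; A hit on E by BP_ThirdPersonCharacter adds HealValue to that character's health and destroys the pickup, using collision hits rather than overlaps.
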(event `self.ReceiveBeginPlay`
  (bind (_direction _floatie) (`Timeline|FloatAnim` :!label _label)
    (:`Update`
      (`SceneComponent.K2_SetRelativeLocation` (`self.e`) _floatie false false))
    (:`Finished`
      (bind (_direction_2 _floatie_2) (`Timeline|Timeline` :!via `ReverseFromEnd`)
        (:`Update`
          (`SceneComponent.K2_SetRelativeLocation` (`self.e`) _floatie_2 false false))
        (:`Finished`
          (goto _label :!via `PlayFromStart`))))))

(event `self.e.OnComponentHit`
  (params (HitComponent :type "PrimitiveComponent Object Reference") (OtherActor :type "Actor Object Reference") (OtherComp :type "PrimitiveComponent Object Reference") (NormalImpulse :type "Vector Structure") (Hit :type "HitResult Structure (by ref)"))
  (bind _asbp_third_person_character (cast `/Game/ThirdPerson/Blueprints/BP_ThirdPersonCharacter` OtherActor))
  (`/Game/ThirdPerson/Blueprints/BP_ThirdPersonCharacter.AddHealth` _asbp_third_person_character (`self.HealValue`))
  (`self.K2_DestroyActor`))

(fn `UserConstructionScript`)