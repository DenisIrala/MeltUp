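; Game mode that handles player game over and respawning at the last checkpoint.
; GameOver disables the player controller's input, waits briefly, then calls RespawnPlayer.
; RespawnPlayer destroys the current character, spawns a fresh BP_ThirdPersonCharacter at the LastCheckpoint's Pos transform regardless of collisions, and has the player controller possess it.
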(event `GameOver`
  (`self.DisableInput` (`GameplayStatics.GetPlayerController` 0) null)
  (`KismetSystemLibrary.Delay` 2.0)
  (`self.RespawnPlayer`))

(event `RespawnPlayer`
  (bind (_returnvalue_location _returnvalue_rotation _returnvalue_scale) (`KismetMathLibrary.BreakTransform` (`SceneComponent.K2_GetComponentToWorld` (`/Game/ThirdPerson/Blueprints/Checkpoint.Pos` (`self.LastCheckpoint`)))))
  (`self.K2_DestroyActor` (`GameplayStatics.GetPlayerCharacter` 0))
  (bind _returnvalue (`|SpawnActorFromClass` "/Game/ThirdPerson/Blueprints/BP_ThirdPersonCharacter.BP_ThirdPersonCharacter_C" (`KismetMathLibrary.MakeTransform` _returnvalue_location _returnvalue_rotation _returnvalue_scale) "AlwaysSpawn" "MultiplyWithRoot" null null))
  (`Controller.Possess` (`GameplayStatics.GetPlayerController` 0) _returnvalue))

(fn `UserConstructionScript`)